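; Base melee attack Gameplay Ability that plays an attack montage when the avatar's weapon manager has an equipped weapon, ending when the montage finishes or is interrupted.
; On authority, gameplay events open and close the weapon's hit scan window, and ending the ability also closes it.
; Opening the window hands the weapon an effect spec carrying set-by-caller damage, so the weapon receives the damage payload from the ability.
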(event Custom|HandleHitScanStart'
  (bind _dmg_mag (Variables|Default|GetDMG%20MAg))
  (bind _returnvalue (Ability|GameplayEffect|AssignTagSetbyCallerMagnitude (Ability|MakeOutgoingGameplayEffectSpec (Variables|GP_Effect|GetEffectClass)) "(TagName=\"Data.Damage\")" _dmg_mag))
  (Default|HitScanStart (stale Ability|EventActivateAbility _eqippedweapon) _returnvalue)
  (Development|PrintString (Utilities|String|ToString(Float) _dmg_mag)))

(event Custom|Handle%20hitScanEnd
  (Default|HitscanEnd (stale Ability|EventActivateAbility _eqippedweapon)))

(event Custom|MontageStarted)

(event Ability|EventActivateAbility
  (bind _returnvalue (Ability|GetAvatarActorfromActorInfo))
  (bind _returnvalue_2 (Actor|GetComponentbyClass _returnvalue "/Game/GAS/Weapons/BP_WeaponManager.BP_WeaponManager_C"))
  (Utilities|IsValid _returnvalue_2
    (:Is%20Valid
      (bind _eqippedweapon (Variables|/Game/GAS/Weapons/BP_WeaponManager.BP_WeaponManager_C|GetEqippedWeapon _returnvalue_2)
        (:then
          (Ability|CommitAbility)
          (bind _attackmontage (Variables|Anim|GetAttackMontage)
            (:then
              (|PlayMontageandWaitProxy "None" _attackmontage 1.0 "None" true 1.0 0.0 true
                (:then
                  (CallFunction|MontageStarted)
                  (Ability|HasAuthority
                    (:True
                      (Ability|Tasks|WaitGameplayEvent "(TagName=\"Event.HitScan.Start\")" 0
                        (:then
                          (Ability|Tasks|WaitGameplayEvent "(TagName=\"Event.HitScan.End\")" 0
                            (:EventReceived
                              (CallFunction|HandleHitScanEnd))))
                        (:EventReceived
                          (CallFunction|HandleHitScanStart'))))))
                (:OnCompleted
                  (Ability|EndAbility :!label _label))
                (:OnInterrupted
                  (goto _label))
                (:OnCancelled
                  (goto _label))))
            (:else
              (Ability|EndAbility :!label _label_2))))
        (:else
          (goto _label_2))))
    (:Is%20Not%20Valid
      (goto _label_2))))

(event Ability|EventOnEndAbility
  (params (bWasCancelled :type Boolean))
  (CallFunction|HandleHitScanEnd))