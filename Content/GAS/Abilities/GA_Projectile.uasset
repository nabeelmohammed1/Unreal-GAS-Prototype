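; GA_Projectile is a Gameplay Ability that fires a projectile from the avatar's equipped weapon.
; On activation it commits without checking the result, then reads the equipped weapon from the avatar's BP_WeaponManager component.
; It spawns ProjectileClass at the weapon's TraceEnd, using the avatar's rotation and ownership.
; EndAbility runs only after that spawn, so a missing manager or weapon leaves the ability active.
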(event Ability|EventActivateAbility
  (bind _returnvalue (Ability|GetAvatarActorfromActorInfo))
  (bind _returnvalue_2 (Actor|GetComponentbyClass _returnvalue "/Game/GAS/Weapons/BP_WeaponManager.BP_WeaponManager_C"))
  (Ability|CommitAbility)
  (Utilities|IsValid _returnvalue_2
    (:Is%20Valid
      (bind _eqippedweapon (Variables|/Game/GAS/Weapons/BP_WeaponManager.BP_WeaponManager_C|GetEqippedWeapon _returnvalue_2)
        (:then
          (Game|SpawnActorfromClass (Variables|Default|GetProjectile%20Class) (Math|Transform|MakeTransform (Transformation|GetWorldLocation (Variables|/Game/GAS/Weapons/BP_Weapon_Base.BP_Weapon_Base_C|GettraceEnd _eqippedweapon)) (Transformation|GetActorRotation _returnvalue) "1.000000,1.000000,1.000000") "Undefined" "MultiplyWithRoot" _returnvalue 0)
          (Ability|EndAbility))
        (:else)))))

(event Ability|EventOnEndAbility
  (params (bWasCancelled :type Boolean)))