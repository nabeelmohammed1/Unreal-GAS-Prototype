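; Base Gameplay Ability for shooting a projectile, timed to a shoot montage.
; On the montage's Event.ShootProjectile gameplay event it takes an instant single-line-trace target, then spawns the projectile on authority aimed at the hit point, passing a damage effect spec with SetByCaller magnitude.
; The spawn point comes from the weapon manager's equipped weapon, falling back to the avatar's location.
; The ability ends when the montage completes, is interrupted or is cancelled.
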(event Ability|EventActivateAbility
  (|PlayMontageandWaitProxy "None" (Variables|Default|Getshoot%20Montage) 1.0 "None" true 1.0 0.0 true
    (:then
      (Ability|Tasks|WaitGameplayEvent "(TagName=\"Event.ShootProjectile\")" 0
        (:EventReceived
          (bind _data (|WaitTargetData :ConfirmationType "Instant" :Class "/Script/GameplayAbilities.GameplayAbilityTargetActor_SingleLineTrace" :TraceProfile "(Name=\"NoCollision\")" :StartLocation (Class|GameplayAbility|MakeTargetLocationInfofromOwnerActor) :ReticleClass 0)
            (:ValidData
              (bind _returnvalue (Ability|GameplayEffect|AssignTagSetbyCallerMagnitude (Ability|MakeOutgoingGameplayEffectSpec (Variables|Default|GetDmgClass)) "(TagName=\"Data.Damage\")" (Variables|Default|GetDmgMag)))
              (bind _location (CallFunction|GetSpawnLocation))
              (|SpawnActor 0 _location "0, 0, 0" (Variables|Default|GetClass) true (Variables|Default|GetSpeed) (Class|AbilitySystemBlueprintLibrary|GetTargetDataEndPoint _data) _returnvalue (.AsGASCharacter%20Base (Utilities|Casting|CastToGASCharacterBase (Ability|GetAvatarActorfromActorInfo)))))))))
    (:OnCompleted
      (Ability|EndAbility :!label _label))
    (:OnInterrupted
      (goto _label))
    (:OnCancelled
      (goto _label))))

(event Ability|EventOnEndAbility
  (params (bWasCancelled :type Boolean)))

(fn GetSpawnLocation
  (bind _returnvalue (Ability|GetAvatarActorfromActorInfo))
  (bind _returnvalue_2 (Actor|GetComponentbyClass _returnvalue "/Game/GAS/Weapons/BP_WeaponManager.BP_WeaponManager_C"))
  (Utilities|IsValid _returnvalue_2
    (:Is%20Valid
      (bind _eqippedweapon (Variables|/Game/GAS/Weapons/BP_WeaponManager.BP_WeaponManager_C|GetEqippedWeapon _returnvalue_2)
        (:then
          (bind _location (Default|GetSpawnpoint _eqippedweapon))
          (if (Utilities|Operators|NotEqual(!=) :A _location)
            (return _location)
            (else
              _)))
        (:else
          _)))
    (:Is%20Not%20Valid
      _))
  (return (Transformation|GetActorLocation (Ability|GetAvatarActorfromActorInfo))))