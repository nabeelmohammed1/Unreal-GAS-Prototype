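; Base GAS weapon that detects hits over a start-to-end window and applies a supplied gameplay effect to what it strikes.
; HitScanStart stores the effect spec, clears the hit list and starts a looping timer at about 30 Hz; HitscanEnd clears it.
; HitScan sphere-traces Pawns between TraceStart and TraceEnd, ignoring the Instigator.
; Each actor with an ability system component receives the effect once per window.
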(event Custom|HitScan
  (bind _outhits (Collision|MultiSphereTraceForObjects (Transformation|GetWorldLocation (Variables|Default|GettraceStart)) (Transformation|GetWorldLocation (Variables|Default|GettraceEnd)) (Variables|Default|GetHitScanRadius) (Utilities|Array|MakeArray "ObjectTypeQuery3") false (Utilities|Array|MakeArray (Variables|Actor|GetInstigator)) "None"))
  (for _array_element _outhits
    (Utilities|IsValid (Ability|GetAbilitySystemComponent (.HitActor (Collision|BreakHitResult _array_element)))
      (:Is%20Valid
        (if (not (Utilities|Array|ContainsItem (Variables|Default|GetHitactors) (.HitActor (Collision|BreakHitResult _array_element))))
          (Utilities|Array|AddUnique (Variables|Default|GetHitactors) (.HitActor (Collision|BreakHitResult _array_element)))
          (GameplayEffects|ApplyGameplayEffectSpecToSelf (Ability|GetAbilitySystemComponent (.HitActor (Collision|BreakHitResult _array_element))) (Variables|Default|GetEffect%20Spec%20Handle)))))))

(event Custom|HitScanStart
  (params (EffectSpecHandle :type Gameplay%20Effect%20Spec%20Handle%20Structure))
  (Variables|Default|SetEffect%20Spec%20Handle EffectSpecHandle)
  (Utilities|Array|Clear (Variables|Default|GetHitactors))
  (bind _returnvalue (Utilities|Time|SetTimerbyEvent (EventDispatchers|CreateEvent :!event Custom|HitScan) 0.033333 true)))

(event Custom|HitscanEnd
  (Utilities|Time|ClearandInvalidateTimerbyHandle (stale Custom|HitScanStart _returnvalue)))

(fn ConstructionScript)