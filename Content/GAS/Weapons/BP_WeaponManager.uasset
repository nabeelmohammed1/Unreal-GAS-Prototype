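; Weapon manager component for a GAS character that spawns starting weapons on the server, attaches them to stowed sockets, and toggles equipping by class.
; Equipping grants the weapon's abilities; unequipping removes them and restores the unarmed config.
; Each weapon config drives anim class, movement settings and montages, whose notify or interruption triggers the socket swap.
; An OnRep on the equipped weapon reapplies the equipped or unarmed state on clients.
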(event Custom|EquipWeapon
  (params (WeaponClass :type BP%20Weapon%20Base%20Class%20Reference))
  (Variables|Default|GetOwningChar
    (:then
      (bind _eqippedweapon (Variables|Default|GetEqippedWeapon)
        (:then
          (if (== (Utilities|GetClass _eqippedweapon) WeaponClass)
            (CallFunction|UnequipWeapon)
            (else
              (CallFunction|UnequipWeapon)
              (bind _stowedweapon (CallFunction|GetStowedweaponbyclass WeaponClass :!label _label))
              (Utilities|IsValid _stowedweapon
                (:Is%20Valid
                  (bind _output_get (Variables|Default|SetEqippedWeapon _stowedweapon))
                  (bind _returnvalue (Class|GASCharacterBase|GrantAbilities (Variables|Default|GetOwningChar) (.abilityToGrant (Utilities|Struct|BreakS_WeaponData (Variables|/Game/GAS/Weapons/BP_Weapon_Base.BP_Weapon_Base_C|GetWeaponConfig _output_get)))))
                  (Variables|Default|SetAbiltiyGrantedPerWeapon _returnvalue)
                  (CallFunction|SetProperties))))))
        (:else
          (goto _label))))
    (:else)))

(event Custom|UnequipWeapon
  (bind _eqippedweapon (Variables|Default|GetEqippedWeapon)
    (:then
      (Class|GASCharacterBase|RemoveAbilities (Variables|Default|GetOwningChar) (Variables|Default|GetAbiltiyGrantedPerWeapon))
      (Variables|Default|SetPreviouslyEqupped _eqippedweapon)
      (Variables|Default|SetEqippedWeapon 0)
      (CallFunction|SetUnarmed))
    (:else)))

(event Custom|giveWeapon
  (params (weapon :type BP%20Weapon%20Base%20Class%20Reference))
  (bind _returnvalue (Game|SpawnActorfromClass weapon (Math|Transform|MakeTransform "0, 0, 0" "0, 0, 0" "1.000000,1.000000,1.000000") "Undefined" "MultiplyWithRoot" 0 (Variables|Default|GetOwningChar)))
  (Utilities|Array|AddUnique (Variables|Default|GetStowedWeapons) _returnvalue)
  (Transformation|AttachComponentToComponent _returnvalue (Variables|/Script/Engine.Character|GetMesh (Variables|Default|GetOwningChar)) (Utilities|Struct|BreakS_WeaponData (Variables|/Game/GAS/Weapons/BP_Weapon_Base.BP_Weapon_Base_C|GetWeaponConfig _returnvalue)) "KeepRelative" "KeepRelative" "KeepRelative" true))

(event Custom|Set%20Properties
  (bind _owningchar (Variables|Default|GetOwningChar))
  (bind _charactermovement (Variables|/Script/Engine.Character|GetCharacterMovement _owningchar))
  (Variables|Default|GetEqippedWeapon
    (:then
      (Components|SkeletalMesh|SetAnimInstanceClass (Variables|/Script/Engine.Character|GetMesh (Variables|Default|GetOwningChar)) (.AnimClass (Utilities|Struct|BreakS_WeaponData (Variables|/Game/GAS/Weapons/BP_Weapon_Base.BP_Weapon_Base_C|GetWeaponConfig (stale Custom|EquipWeapon _output_get)))))
      (Variables|/Script/Engine.CharacterMovementComponent|SetMaxWalkSpeed _charactermovement (.maxwalkspeed (.MovementProp (Utilities|Struct|BreakS_WeaponData (Variables|/Game/GAS/Weapons/BP_Weapon_Base.BP_Weapon_Base_C|GetWeaponConfig (stale Custom|EquipWeapon _output_get))))))
      (Variables|/Script/Engine.CharacterMovementComponent|SetbOrientRotationToMovement _charactermovement (.orientrotationmovement (.MovementProp (Utilities|Struct|BreakS_WeaponData (Variables|/Game/GAS/Weapons/BP_Weapon_Base.BP_Weapon_Base_C|GetWeaponConfig (stale Custom|EquipWeapon _output_get))))))
      (Variables|/Script/Engine.CharacterMovementComponent|SetbUseControllerDesiredRotation _charactermovement (.usecontrollerdesired (.MovementProp (Utilities|Struct|BreakS_WeaponData (Variables|/Game/GAS/Weapons/BP_Weapon_Base.BP_Weapon_Base_C|GetWeaponConfig (stale Custom|EquipWeapon _output_get))))))
      (bind _notifyname (Animation|Montage|PlayMontage (Variables|/Script/Engine.Character|GetMesh _owningchar) (.Equpmontage (Utilities|Struct|BreakS_WeaponData (Variables|/Game/GAS/Weapons/BP_Weapon_Base.BP_Weapon_Base_C|GetWeaponConfig (stale Custom|EquipWeapon _output_get)))) 1.0 0.0 "None" false)
        (:OnInterrupted
          _)
        (:OnNotifyBegin
          (switch name _notifyname
            (:Equip
              _))))
      (Transformation|AttachComponentToComponent (Variables|Default|GetEqippedWeapon) (Variables|/Script/Engine.Character|GetMesh (Variables|Default|GetOwningChar)) (.Socket (Utilities|Struct|BreakS_WeaponData (Variables|/Game/GAS/Weapons/BP_Weapon_Base.BP_Weapon_Base_C|GetWeaponConfig (stale Custom|EquipWeapon _output_get)))) "SnapToTarget" "SnapToTarget" "SnapToTarget" true))
    (:else)))

(event Custom|Set%20Unarmed
  (bind _owningchar (Variables|Default|GetOwningChar))
  (bind _unarmedweaponcongifg (Variables|Default|GetunarmedWeaponCongifg))
  (bind _previouslyequpped (Variables|Default|GetPreviouslyEqupped))
  (bind _owningchar_2 (Variables|Default|GetOwningChar))
  (bind (_animclass _movementprop) (Utilities|Struct|BreakS_WeaponData _unarmedweaponcongifg))
  (bind _charactermovement (Variables|/Script/Engine.Character|GetCharacterMovement _owningchar))
  (bind _mesh (Variables|/Script/Engine.Character|GetMesh _owningchar_2))
  (bind (_maxwalkspeed _orientrotationmovement _usecontrollerdesired) (Utilities|Struct|BreakS_MovementProperties _movementprop))
  (Components|SkeletalMesh|SetAnimInstanceClass _mesh _animclass)
  (bind _notifyname (Animation|Montage|PlayMontage _mesh (Utilities|Struct|BreakS_WeaponData (Variables|/Game/GAS/Weapons/BP_Weapon_Base.BP_Weapon_Base_C|GetWeaponConfig (Variables|Default|GetPreviouslyEqupped))) 1.0 0.0 "None" false)
    (:OnInterrupted
      _)
    (:OnNotifyBegin
      (switch name _notifyname
        (:Unequip
          _))))
  (Transformation|AttachComponentToComponent _previouslyequpped (Variables|/Script/Engine.Character|GetMesh (Variables|Default|GetOwningChar)) (Utilities|Struct|BreakS_WeaponData (Variables|/Game/GAS/Weapons/BP_Weapon_Base.BP_Weapon_Base_C|GetWeaponConfig _previouslyequpped)) "SnapToTarget" "SnapToTarget" "SnapToTarget" true)
  (Variables|/Script/Engine.CharacterMovementComponent|SetMaxWalkSpeed _charactermovement _maxwalkspeed)
  (Variables|/Script/Engine.CharacterMovementComponent|SetbOrientRotationToMovement _charactermovement _orientrotationmovement)
  (Variables|/Script/Engine.CharacterMovementComponent|SetbUseControllerDesiredRotation _charactermovement _usecontrollerdesired))

(event EventBeginPlay
  (bind _asgascharacter_base (Utilities|Casting|CastToGASCharacterBase (Components|GetOwner)))
  (Variables|Default|SetOwningChar _asgascharacter_base)
  (Networking|SwitchHasAuthority
    (:Authority
      (for _array_element (Variables|Default|GetstartingWeapons)
        (CallFunction|GiveWeapon _array_element)))))

(fn GetStowedweaponbyclass
  (params (weaponclass :type BP%20Weapon%20Base%20Class%20Reference))
  (for _array_element (Variables|Default|GetStowedWeapons)
    (if (== (Utilities|GetClass _array_element) weaponclass)
      (return _array_element))))

(fn OnRepEqippedWeapon
  (Variables|Default|GetEqippedWeapon
    (:then
      (CallFunction|SetProperties))
    (:else
      (CallFunction|SetUnarmed))))